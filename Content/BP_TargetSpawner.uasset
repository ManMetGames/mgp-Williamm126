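; BP_TargetSpawner is an actor that continuously spawns BP_Target actors along a spline path.
; On BeginPlay it spawns a target at the SpawnPoint component's transform and passes SplinePath to the target's SplineToFollow.
; It then waits a random delay between MinSpawnDelay and MaxSpawnDelay and calls SpawnTarget again, forming an endless self-repeating loop.
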(event `self.ReceiveBeginPlay`
  (`self.Spawn Target`))

(event `Spawn Target`
  (bind _returnvalue (`|SpawnActorFromClass` "/Game/BP_Target.BP_Target_C" (`SceneComponent.K2_GetComponentToWorld` (`self.SpawnPoint`)) "Undefined" "MultiplyWithRoot" null null))
  (set `/Game/BP_Target.Spline To Follow` (`self.SplinePath`) _returnvalue)
  (`KismetSystemLibrary.Delay` (`KismetMathLibrary.RandomFloatInRange` (`self.MinSpawnDelay`) (`self.MaxSpawnDelay`)))
  (`self.Spawn Target`))

(fn `UserConstructionScript`)
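; BP_Target is a numbered target that travels along a spline and costs the player a life if it reaches the end.
; It spawns with a random multiple of 3 or 5, which sets its text, colour and timeline-driven travel time.
; LeftClickHit divides by 3 and RightClickHit by 5 when divisible, destroying it once neither factor remains.
; The older projectile-overlap handler is never bound.
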(event `Move Object`
  (bind _spline (`/Game/BP_Splinepath.Spline` (`self.Spline To Follow`)))
  (`TimelineComponent.SetPlayRate` (`self.T_Move`) (/ 1.0 (`self.Time To Complete`)))
  (bind (_direction _move_track) (`Timeline|T_Move`)
    (:`Update`
      (bind _returnvalue (`KismetMathLibrary.Lerp` 0.0 (`SplineComponent.GetSplineLength` _spline) _move_track))
      (`self.K2_SetActorLocationAndRotation` (`SplineComponent.GetLocationAtDistanceAlongSpline` _spline _returnvalue "World") (`SplineComponent.GetRotationAtDistanceAlongSpline` _spline _returnvalue "World")))
    (:`Finished`
      (bind _asbp_third_person_character (cast `/Game/ThirdPerson/Blueprints/BP_ThirdPersonCharacter` (`GameplayStatics.GetPlayerCharacter` 0)))
      (`/Game/ThirdPerson/Blueprints/BP_ThirdPersonCharacter.LoseLife` _asbp_third_person_character)
      (`self.K2_DestroyActor`))))

(event `self.ReceiveBeginPlay`
  (if (`KismetMathLibrary.RandomBool`)
    (set `self.TargetNumber` (* (`KismetMathLibrary.RandomIntegerInRange` 1 5500) 5))
    (`self.Refresh Target`)
    (else
      (set `self.TargetNumber` (* (`KismetMathLibrary.RandomIntegerInRange` 1 3300) 3))
      (`self.Refresh Target`))))

(event `self.ReceiveHit`
  (params (MyComp :type "PrimitiveComponent Object Reference") (Other :type "Actor Object Reference") (OtherComp :type "PrimitiveComponent Object Reference") (bSelfMoved :type Boolean) (HitLocation :type "Vector Structure") (HitNormal :type "Vector Structure") (NormalImpulse :type "Vector Structure") (Hit :type "HitResult Structure (by ref)"))
  (`GameplayStatics.SpawnEmitterAtLocation` "/Engine/Tutorial/SubEditors/TutorialAssets/TutorialParticleSystem.TutorialParticleSystem" HitLocation :!label _label)
  (`GameplayStatics.PlaySoundAtLocation` "/Engine/EngineSounds/1kSineTonePing.1kSineTonePing" HitLocation (struct) 1.0 1.0 0.0 null null null null)
  (`self.K2_DestroyActor`))

(event `Refresh Target`
  (`TextRenderComponent.K2_SetText` (`self.TextRender`) (`KismetTextLibrary.Conv_IntToText` (`self.TargetNumber`)))
  (`TextRenderComponent.K2_SetText` (`self.TextRender1`) (`KismetTextLibrary.Conv_IntToText` (`self.TargetNumber`)))
  (`TextRenderComponent.K2_SetText` (`self.TextRender2`) (`KismetTextLibrary.Conv_IntToText` (`self.TargetNumber`)))
  (`TextRenderComponent.K2_SetText` (`self.TextRender3`) (`KismetTextLibrary.Conv_IntToText` (`self.TargetNumber`)))
  (`MeshComponent.SetVectorParameterValueOnMaterials` (`self.Cube`) "TargetColour" (`KismetMathLibrary.Conv_LinearColorToVector` (`TargetColourLibrary.GetColourForTargetNumber` (`self.TargetNumber`))))
  (set `self.Time To Complete` (`KismetMathLibrary.Conv_IntToDouble` (+ (/ (`self.TargetNumber`) 500) 4)))
  (`self.Move Object`))

(event `OnComponentBeginOverlap_Event`
  (params (OverlappedComponent :type "PrimitiveComponent Object Reference") (OtherActor :type "Actor Object Reference") (OtherComp :type "PrimitiveComponent Object Reference") (OtherBodyIndex :type Integer) (bFromSweep :type Boolean) (SweepResult :type "HitResult Structure (by ref)"))
  (cast `/Game/Left_Click_Projectile` OtherActor
    (:`then`
      (goto _label))
    (:`CastFailed`
      (cast `/Game/Right_Click_projectile` OtherActor)
      (`KismetSystemLibrary.PrintString` "right click hit")
      (bind _output_get (set `self.TargetNumber` (/ (`self.TargetNumber`) 5)))
      (`TextRenderComponent.K2_SetText` (`self.TextRender`) (`KismetTextLibrary.Conv_IntToText` _output_get))
      (`TextRenderComponent.K2_SetText` (`self.TextRender1`) (`KismetTextLibrary.Conv_IntToText` _output_get))
      (`TextRenderComponent.K2_SetText` (`self.TextRender2`) (`KismetTextLibrary.Conv_IntToText` _output_get))
      (`TextRenderComponent.K2_SetText` (`self.TextRender3`) (`KismetTextLibrary.Conv_IntToText` _output_get)))))

(event `RightClickHit`
  (bind _targetnumber (`self.TargetNumber`))
  (if (== (mod _targetnumber 5) 0)
    (bind _output_get (set `self.TargetNumber` (/ _targetnumber 5)))
    (`TextRenderComponent.K2_SetText` (`self.TextRender`) (`KismetTextLibrary.Conv_IntToText` _output_get))
    (`TextRenderComponent.K2_SetText` (`self.TextRender1`) (`KismetTextLibrary.Conv_IntToText` _output_get))
    (`TextRenderComponent.K2_SetText` (`self.TextRender2`) (`KismetTextLibrary.Conv_IntToText` _output_get))
    (`TextRenderComponent.K2_SetText` (`self.TextRender3`) (`KismetTextLibrary.Conv_IntToText` _output_get))
    (`MeshComponent.SetVectorParameterValueOnMaterials` (`self.Cube`) "TargetColour" (`KismetMathLibrary.Conv_LinearColorToVector` (`TargetColourLibrary.GetColourForTargetNumber` _targetnumber)))
    (if (not (or (== (mod (`self.TargetNumber`) 3) 0) (== (mod (`self.TargetNumber`) 5) 0)))
      (`self.K2_DestroyActor`))))

(event `LeftClickHit`
  (bind _targetnumber (`self.TargetNumber`))
  (if (== (mod _targetnumber 3) 0)
    (bind _output_get (set `self.TargetNumber` (/ _targetnumber 3)))
    (`TextRenderComponent.K2_SetText` (`self.TextRender`) (`KismetTextLibrary.Conv_IntToText` _output_get))
    (`TextRenderComponent.K2_SetText` (`self.TextRender1`) (`KismetTextLibrary.Conv_IntToText` _output_get))
    (`TextRenderComponent.K2_SetText` (`self.TextRender2`) (`KismetTextLibrary.Conv_IntToText` _output_get))
    (`TextRenderComponent.K2_SetText` (`self.TextRender3`) (`KismetTextLibrary.Conv_IntToText` _output_get))
    (`MeshComponent.SetVectorParameterValueOnMaterials` (`self.Cube`) "TargetColour" (`KismetMathLibrary.Conv_LinearColorToVector` (`TargetColourLibrary.GetColourForTargetNumber` _targetnumber)))
    (if (not (or (== (mod (`self.TargetNumber`) 3) 0) (== (mod (`self.TargetNumber`) 5) 0)))
      (`self.K2_DestroyActor`))))

(fn `UserConstructionScript`
  (`StaticMeshComponent.SetStaticMesh` (`self.Cube`) (`self.Object Mesh`)))